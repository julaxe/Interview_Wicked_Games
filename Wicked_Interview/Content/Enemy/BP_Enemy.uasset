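; BP_Enemy is an enemy Blueprint that keeps track of its position along a looping list of patrol points.
; GoToNextPatrolPoint increments the current index and wraps it with a modulo on the list length.
; GetPatrolPointLocation returns the entry at that index, while the construction script only calls its parent.
; The file contains no movement logic, only this index bookkeeping.
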(fn `GetPatrolPointLocation`
  (returns (CurrentPatrolPointLocation :type "Actor Object Reference"))
  (return (`|GetArrayItem` (`self.PatrolPoints`) (`self.CurrentPatrolPoint`))))

(fn `GoToNextPatrolPoint`
  (bind _result (`/Engine/EditorBlueprintResources/StandardMacros.IncrementInt` (`self.CurrentPatrolPoint`))
    (:`  `
      (set `self.CurrentPatrolPoint` (mod _result (`KismetArrayLibrary.Array_Length` (`self.PatrolPoints`)))))))

(fn `UserConstructionScript`
  (`parent.UserConstructionScript`))